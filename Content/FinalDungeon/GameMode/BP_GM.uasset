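; Game mode for the final dungeon that moves the player between streamed levels and gates portals behind clearing monsters.
; OpenStreamLevel removes input mappings, unloads the current level, loads the next with camera fades, then restores input.
; For levels not cleared in BP_GameState, it spawns BP_SpawnSpawners, hides portals and polls on a looping timer until no normal monsters remain.
; It also handles player teleports and starts players at "Start1".
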(event `OpenStreamLevel`
  (params (ToGoLevel :type Name) (CurrentLevel :type Name))
  (`self.UnPossess`
    (:`end`
      (`self.UnLoadLevel` CurrentLevel
        (:`end`
          (`self.OpenNewLevel` ToGoLevel
            (:`end`
              (`self.LoadGameManager` ToGoLevel))))))))

(event `TeleportPlayer`
  (params (DestLocation :type "Vector Structure") (DestRotation :type "Rotator Structure"))
  (`self.K2_TeleportTo` (`GameplayStatics.GetPlayerPawn` 0) DestLocation DestRotation))

(event `self.ReceiveBeginPlay`)

(fn `ChoosePlayerStart`
  (params (Player :type "Controller Object Reference"))
  (returns (ReturnValue :type "Actor Object Reference"))
  (return (`self.K2_FindPlayerStart` Player "Start1")))

(fn `HasClear`
  (bind _outactors (`GameplayStatics.GetAllActorsOfClass` "/Game/FinalDungeon/Monsters/BP_NormalMonsterBase.BP_NormalMonsterBase_C"))
  (if (== (`KismetArrayLibrary.Array_Length` _outactors) 0)
    (`KismetSystemLibrary.K2_ClearTimer` null "HasClear")
    (for _array_element (`self.Portals`)
      (`self.SetActorEnableCollision` _array_element true)
      (`self.SetActorHiddenInGame` _array_element false))))

(fn `SpawnSpawner`
  (`|SpawnActorFromClass` "/Game/FinalDungeon/Levels/Actors/BP_SpawnSpawners.BP_SpawnSpawners_C" (`KismetMathLibrary.MakeTransform` (0.0 0.0 0.0)) "Undefined" "MultiplyWithRoot" null null))

(fn `UnVisiblePortals`
  (bind _outactors (`GameplayStatics.GetAllActorsOfClass` "/Game/FinalDungeon/Levels/Actors/BP_Portal.BP_Portal_C"))
  (bind _output_get (set `self.Portals` _outactors))
  (for _array_element _output_get
    (`self.SetActorEnableCollision` _array_element false)
    (`self.SetActorHiddenInGame` _array_element true)))

(fn `UserConstructionScript`)