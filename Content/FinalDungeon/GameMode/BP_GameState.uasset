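; Game state for the FinalDungeon mode that tracks the cleared status of each stage level.
; On BeginPlay it copies every DT_Stage row into LevelStates and gathers all PlayerStart actors into PlayerStarts.
; StoreIsClear takes a level name and overwrites each entry with a matching StreamName as cleared.
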(event `self.ReceiveBeginPlay`
  (`|ExecutionSequence`
    (:`then_0`
      (bind _outrownames (`DataTableFunctionLibrary.GetDataTableRowNames` "/Game/FinalDungeon/Levels/DT_Stage.DT_Stage"))
      (for _array_element _outrownames
        (bind _returnvalue (`|GetDataTableRow` "/Game/FinalDungeon/Levels/DT_Stage.DT_Stage" _array_element)
          (:`then`
            (`KismetArrayLibrary.Array_Add` (`self.LevelStates`) _returnvalue)))))
    (:`then_1`
      (bind _outactors (`GameplayStatics.GetAllActorsOfClass` "/Script/Engine.PlayerStart"))
      (for _array_element_2 _outactors
        (`KismetArrayLibrary.Array_Add` (`self.PlayerStarts`) _array_element_2)))))

(event `StoreIsClear`
  (params (LevelName :type Name))
  (bind _levelstates (`self.LevelStates`))
  (for (_array_element _array_index) _levelstates
    (if (== (`.StreamName_4_63B69CA04D2ECC365BCBBA91C01096E9` (break `/Game/FinalDungeon/Levels/ST_Stage` _array_element)) LevelName)
      (`KismetArrayLibrary.Array_Set` _levelstates _array_index (make `/Game/FinalDungeon/Levels/ST_Stage` true LevelName)))))

(fn `UserConstructionScript`)