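; BP_NormalMonsterBase is the base Blueprint for normal monsters in the Final Dungeon, providing AI-driven attack state and movement speed helpers.
; UpdateAITick reads the NormalMonsterState enum from the AI controller's Blackboard and sets IsAttacking in the Attack state.
; When an AI controller possesses it, it binds to the anim instance's montage-ended event, which clears IsAttacking.
; Separate functions switch max walk speed between chase and patrol values.
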(event `self.ReceivePossessed`
  (params (NewController :type "Controller Object Reference"))
  (cast `AIController` NewController)
  (add `AnimInstance.OnMontageEnded` (`SkeletalMeshComponent.GetAnimInstance` (`self.Mesh`)) (`|CreateDelegate` :!event `MontageEnd`)))

(event `MontageEnd`
  (params (Montage :type "AnimMontage Object Reference") (bInterrupted :type Boolean))
  (set `self.IsAttacking` false))

(fn `UpdateAITick`
  (bind _asaicontroller (cast `AIController` (`self.GetController`)))
  (bind _output_get (set `self.NormalMonsterState` (cast `/Game/FinalDungeon/Monsters/NormalAI/EN_NormalMonsterStates` (`BlackboardComponent.GetValueAsEnum` (`AIBlueprintHelperLibrary.GetBlackboard` _asaicontroller) "NormalMonsterState"))))
  (switch `/Game/FinalDungeon/Monsters/NormalAI/EN_NormalMonsterStates` _output_get
    (:`NewEnumerator2`
      (if (not (`self.IsAttacking`))
        (set `self.IsAttacking` true)))))

(fn `UpdateChaseSpeed`
  (set `CharacterMovementComponent.MaxWalkSpeed` (`self.ChaseSpeed`) (`self.CharacterMovement`)))

(fn `UpdatePatrolSpeed`
  (set `CharacterMovementComponent.MaxWalkSpeed` (`self.PatrolSpeed`) (`self.CharacterMovement`)))

(fn `UserConstructionScript`)