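; Anim notify for the Khaimera boss that deals combo attack damage when an animation reaches it.
; It runs a sphere overlap for pawns at a fixed offset in front of the boss, sized by AttackRadius and ignoring the boss itself.
; Each overlapped actor takes fixed damage with Khaimera as the causer, and a debug sphere draws the hit area.
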(fn `Received_Notify`
  (params (MeshComp :type "SkeletalMeshComponent Object Reference") (Animation :type "AnimSequenceBase Object Reference") (EventReference :type "AnimNotifyEventReference Structure (by ref)"))
  (returns (ReturnValue :type Boolean))
  (bind _asbp_khaimera (cast `/Game/FinalDungeon/Monsters/Boss_Khaimera/BP_Khaimera` (`ActorComponent.GetOwner` MeshComp)))
  (bind _returnvalue (+ (`Actor.K2_GetActorLocation` _asbp_khaimera) (* (`Actor.GetActorForwardVector` _asbp_khaimera) 300.0)))
  (bind _outactors (`KismetSystemLibrary.SphereOverlapActors` _returnvalue (`self.AttackRadius`) (`|MakeArray` "ObjectTypeQuery3" :!type "EObjectTypeQuery Enum") null (`|MakeArray` _asbp_khaimera :!type "Actor Object Reference")))
  (`KismetSystemLibrary.DrawDebugSphere` _returnvalue (`self.AttackRadius`))
  (for _array_element _outactors
    (`GameplayStatics.ApplyDamage` _array_element 10.0 null _asbp_khaimera))
  (return false))