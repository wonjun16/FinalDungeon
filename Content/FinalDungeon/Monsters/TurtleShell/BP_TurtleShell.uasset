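; TurtleShell monster Blueprint that loads its stats by name and handles attacking, damage reactions and death.
; On AI possession, a looping timer polls the blackboard state; Attack triggers a random montage and a short-lived collision actor in front, gated by IsAttacking.
; Damage plays a hit montage unless attacking.
; At zero HP it disables collision, plays a slowed death montage and schedules destruction.
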(event `self.ReceiveBeginPlay`
  (`self.InitializeMonsterStat` "TurtleShell")
  (`parent.ReceiveBeginPlay`))

(event `self.ReceivePossessed`
  (params (NewController :type "Controller Object Reference"))
  (cast `AIController` NewController)
  (add `AnimInstance.OnMontageEnded` (`SkeletalMeshComponent.GetAnimInstance` (`self.Mesh`)) (`|CreateDelegate` :!event `MontageEnd`))
  (`KismetSystemLibrary.K2_SetTimer` null "UpdateAITick" 0.01 true))

(event `self.ReceiveAnyDamage`
  (params (Damage :type "Float (single-precision)") (DamageType :type "DamageType Object Reference") (InstigatedBy :type "Controller Object Reference") (DamageCauser :type "Actor Object Reference"))
  (bind _monsterstat_hp (break `/Game/FinalDungeon/Monsters/Stats/ST_NormalMonsterStat` (`self.MonsterStat`)))
  (`parent.ReceiveAnyDamage` Damage DamageType InstigatedBy DamageCauser)
  (`|ExecutionSequence`
    (:`then_0`
      (if (not (`self.IsAttacking`))
        (`self.PlayAnimMontage` (`self.DemagedMontage`))))
    (:`then_1`
      (if (<= _monsterstat_hp 0)
        (`PrimitiveComponent.SetCollisionEnabled` (`self.CapsuleComponent`) "NoCollision")
        (`PrimitiveComponent.SetCollisionEnabled` (`self.Mesh`) "NoCollision")
        (`self.PlayAnimMontage` (`self.DieMontage`) 0.5)
        (`KismetSystemLibrary.K2_SetTimer` null "DestroyMonster" 1.0)))))

(fn `UpdateAITick`
  (bind _capsulecomponent (`self.CapsuleComponent`))
  (bind _asaicontroller (cast `AIController` (`self.GetController`)))
  (bind _output_get (set `self.NormalMonsterState` (cast `/Game/FinalDungeon/Monsters/NormalAI/EN_NormalMonsterStates` (`BlackboardComponent.GetValueAsEnum` (`AIBlueprintHelperLibrary.GetBlackboard` _asaicontroller) "NormalMonsterState"))))
  (switch `/Game/FinalDungeon/Monsters/NormalAI/EN_NormalMonsterStates` _output_get
    (:`NewEnumerator2`
      (if (not (`self.IsAttacking`))
        (set `self.IsAttacking` true)
        (`self.PlayAnimMontage` (`KismetArrayLibrary.Array_Random` (`self.AttackMontages`)))
        (bind _returnvalue (`|SpawnActorFromClass` "/Game/FinalDungeon/Monsters/BP_AttackCollision.BP_AttackCollision_C" (`KismetMathLibrary.MakeTransform` (+ (`SceneComponent.K2_GetComponentLocation` _capsulecomponent) (* (`SceneComponent.GetForwardVector` _capsulecomponent) 50.0))) "Undefined" "MultiplyWithRoot" null self))
        (set `self.AttackCollision` _returnvalue)
        (`KismetSystemLibrary.K2_SetTimer` null "DestroyAttackCollision" 0.05)))))

(fn `UserConstructionScript`
  (`parent.UserConstructionScript`))