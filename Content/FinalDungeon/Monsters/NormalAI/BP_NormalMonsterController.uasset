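; AI controller for normal monsters in the final dungeon, which starts the BT_NormalMonster behavior tree on BeginPlay.
; AI perception updates drive the blackboard: a sensed actor tagged Player becomes TargetActor and switches the NormalMonsterState enum.
; Any other perception update, including losing sight of the player or sensing a non-player, clears the target and resets the state.
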(event `self.ReceiveBeginPlay`
  (`self.RunBehaviorTree` "/Game/FinalDungeon/Monsters/NormalAI/BT_NormalMonster.BT_NormalMonster"))

(event `self.AIPerception.OnTargetPerceptionUpdated`
  (params (Actor :type "Actor Object Reference") (Stimulus :type "AIStimulus Structure"))
  (if (and (`self.ActorHasTag` Actor "Player") (`.bSuccessfullySensed` (break `AIStimulus` Stimulus)))
    (`BlackboardComponent.SetValueAsObject` (`AIBlueprintHelperLibrary.GetBlackboard` null) "TargetActor" Actor)
    (`BlackboardComponent.SetValueAsEnum` (`AIBlueprintHelperLibrary.GetBlackboard` null) "NormalMonsterState" (enumliteral `/Game/FinalDungeon/Monsters/NormalAI/EN_NormalMonsterStates` "NewEnumerator1"))
    (else
      (`BlackboardComponent.SetValueAsObject` (`AIBlueprintHelperLibrary.GetBlackboard` null) "TargetActor" null)
      (`BlackboardComponent.SetValueAsEnum` (`AIBlueprintHelperLibrary.GetBlackboard` null) "NormalMonsterState" (enumliteral `/Game/FinalDungeon/Monsters/NormalAI/EN_NormalMonsterStates` "NewEnumerator0")))))

(fn `UserConstructionScript`)